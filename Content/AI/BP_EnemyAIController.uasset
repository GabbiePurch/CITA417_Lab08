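; Enemy AI controller that runs the BT_Enemy behavior tree when it possesses a pawn.
; Its AI Perception updates feed the TargetActor blackboard key, setting it when player 0's ThirdPersonCharacter is successfully sensed.
; Any other update from a ThirdPersonCharacter, including losing sight or other stimulus of the player, clears the key immediately, while other actor types are ignored.
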(event OnTargetPerceptionUpdated(AIPerception)
  (params (Actor :type Actor%20Object%20Reference) (Stimulus :type AI%20Stimulus%20Structure))
  (bind _returnvalue (AI|GetBlackboard 0))
  (bind _returnvalue_2 (Utilities|Name|MakeLiteralName "TargetActor"))
  (bind _asbp_third_person_character (Utilities|Casting|CastToBP_ThirdPersonCharacter Actor))
  (if (and (== Actor (Game|GetPlayerCharacter 0)) (.bSuccessfullySensed (Utilities|Struct|BreakAIStimulus Stimulus)))
    (AI|Components|Blackboard|SetValueasObject _returnvalue _returnvalue_2 _asbp_third_person_character)
    (else
      (AI|Components|Blackboard|ClearValue _returnvalue _returnvalue_2))))

(event EventBeginPlay)

(event EventTick
  (params (DeltaSeconds :type Float%20%28single-precision%29)))

(event EventPossess
  (params (PossessedPawn :type Pawn%20Object%20Reference))
  (AI|RunBehaviorTree "/Game/AI/BT_Enemy.BT_Enemy"))

(fn ConstructionScript)